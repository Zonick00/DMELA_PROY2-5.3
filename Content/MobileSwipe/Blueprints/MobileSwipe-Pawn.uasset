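; Mobile swipe pawn that detects touch swipe direction and reports it to a DirectionDetector widget, active only while that widget is shown.
; A drag longer than a tenth of viewport height fires once per touch through a DoOnce, reset on release.
; The start-to-stop Atan2 angle is bucketed into 4-way simple, 4-way diagonal or 8-way directions.
; Tick also eases camera FOV toward a target; Escape quits.
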(event Custom|CreateWidget
  (params (LoadData? :type Boolean) (PersonalizacionData :type S%20Data%20Personalizacion%20Item%20Structure))
  (bind _returnvalue (UserInterface|CreateWidget "/Game/MobileSwipe/Widgets/DirectionDetector.DirectionDetector_C" 0 LoadData? PersonalizacionData))
  (bind _output_get (Variables|Default|SetDirection%20Widget _returnvalue))
  (UserInterface|Viewport|AddtoViewport _output_get 0)
  (Variables|Default|SetWidgetInViewport? true))

(event Custom|ModificarVistaCamara
  (params (DeltaTime :type Float%20%28single-precision%29))
  (bind _camera (Variables|Default|GetCamera))
  (bind _targetfieldview (Variables|Default|GetTargetFieldView))
  (bind _fieldofview (Variables|/Script/Engine.CameraComponent|GetFieldOfView _camera))
  (if (not (Math|Float|NearlyEqual(Float) _targetfieldview _fieldofview 0.01))
    (Camera|SetFieldOfView (Variables|Default|GetCamera) (Math|Interpolation|FInterpTo _fieldofview _targetfieldview DeltaTime 5.0))))

(event Custom|DeleteWidget
  (Widget|RemovefromParent (Variables|Default|GetDirection%20Widget))
  (Variables|Default|SetDirection%20Widget 0)
  (Variables|Default|SetWidgetInViewport? false))

(event EventBeginPlay
  (Variables|/Script/Engine.PlayerController|SetbShowMouseCursor (Game|GetPlayerController 0) true)
  (Utilities|FlowControl|Delay 0.1)
  (Variables|Default|SetSwipe%20Lenght (* (/ (.y (Viewport|GetViewportSize)) 1e+02) 1e+01)))

(event EventTick
  (params (DeltaSeconds :type Float%20%28single-precision%29))
  (CallFunction|ModificarVistaCamara DeltaSeconds))

(event Input|KeyboardEvents|Escape
  (params (Key :type Key%20Structure :default "None"))
  (:Pressed
    (Game|QuitGame 0 "Quit" false)))

(event Input|TouchEvents|InputTouch
  (params (Location :type Vector) (FingerIndex :type ETouchIndex%20Enum))
  (bind _returnvalue (Game|GetPlayerController 0))
  (bind (_locationx _locationy) (Class|PlayerController|GetInputTouchState _returnvalue "Touch1"))
  (bind _returnvalue_2 (Math|Vector2D|MakeVector2D _locationx _locationy))
  (:Pressed
    (if (Variables|Default|GetWidgetInViewport?)
      (Variables|Default|SetPressed true)
      (Variables|Default|SetStart _returnvalue_2)))
  (:Released
    (Variables|Default|SetPressed false)
    (goto _label Reset))
  (:Moved
    (if (Variables|Default|GetPressed)
      (if (> (Math|Vector2D|Vector2DLength (- (Variables|Default|GetStart) _returnvalue_2)) (Variables|Default|GetSwipe%20Lenght))
        (Utilities|FlowControl|DoOnce false :!label _label
          (:Completed
            (Variables|Default|SetStop _returnvalue_2)
            (switch Utilities|FlowControl|Switch|SwitchonMobileSwipe-Type (Variables|Default|GetMobile%20Swipe%20-%20Type)
              (:NewEnumerator0
                (|4-WaySwipeMovement(Simple)))
              (:NewEnumerator1
                (|4-WaySwipeMovement(Diagonal)))
              (:NewEnumerator2
                (|8-WaySwipeMovement)))))))))

(fn ConstructionScript)